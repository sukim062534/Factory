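; BP_GameMode is a game mode that populates the level with AI-controlled robots when play begins.
; On BeginPlay it finds all Target actors and spawns a BP_Robot at each one's transform.
; It then seeds each robot's BP_AIController blackboard with the spawn position as HomeLocation and the robot itself as SelfActor.
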(event `self.ReceiveBeginPlay`
  (bind _outactors (`GameplayStatics.GetAllActorsOfClass` "/Game/Blueprint/Item/Target.Target_C"))
  (for _array_element _outactors
    (bind _returnvalue (`|SpawnActorFromClass` "/Game/Blueprint/Robot/BP_Robot.BP_Robot_C" (`self.GetTransform` _array_element) "Undefined" "MultiplyWithRoot" null null))
    (bind _asbp_aicontroller (cast `/Game/Blueprint/Robot/BP_AIController` (`Pawn.GetController` _returnvalue)))
    (bind _blackboard (`AIController.Blackboard` _asbp_aicontroller))
    (`BlackboardComponent.SetValueAsVector` _blackboard (`self.HomeLocation`) (.location (`self.GetTransform` _returnvalue)))
    (`BlackboardComponent.SetValueAsObject` _blackboard (`self.SelfActor `) _returnvalue)))

(fn `UserConstructionScript`)