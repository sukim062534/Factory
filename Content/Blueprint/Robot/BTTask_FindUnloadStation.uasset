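; Behavior tree task that finds and reserves a free unload station for a robot.
; It scans all BP_UnloadStation actors and takes the first one not occupied, marking it occupied and reserved by the robot.
; The station and its RobotArrow location and rotation are written to blackboard keys.
; The task succeeds if a station is found and fails otherwise.
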(event `self.ReceiveExecuteAI`
  (params (OwnerController :type "AIController Object Reference") (ControlledPawn :type "Pawn Object Reference"))
  (set `self.FoundUnloadStation` false)
  (bind _outactors (`GameplayStatics.GetAllActorsOfClass` "/Game/Blueprint/Item/BP_UnloadStation.BP_UnloadStation_C"))
  (for _array_element _outactors
    (bind _boccupied (message `/Game/Blueprint/BPI_Interactable.IsOccupied` _array_element))
    (if (not _boccupied)
      (`BTFunctionLibrary.SetBlackboardValueAsObject` (`self.TargetStation`) _array_element)
      (bind _asbp_unload_station (cast `/Game/Blueprint/Item/BP_UnloadStation` _array_element))
      (set `/Game/Blueprint/Item/BP_UnloadStation.bIsOccupied` true _asbp_unload_station)
      (bind _asbp_robot (cast `/Game/Blueprint/Robot/BP_Robot` ControlledPawn))
      (set `/Game/Blueprint/Item/BP_UnloadStation.ReservedBy` _asbp_robot _asbp_unload_station)
      (bind _robotarrow (`/Game/Blueprint/Item/BP_UnloadStation.RobotArrow` _asbp_unload_station))
      (`BTFunctionLibrary.SetBlackboardValueAsVector` (`self.TargetLocationKey`) (`SceneComponent.K2_GetComponentLocation` _robotarrow))
      (`BTFunctionLibrary.SetBlackboardValueAsRotator` (`self.TargetRotation`) (`SceneComponent.K2_GetComponentRotation` _robotarrow))
      (set `self.FoundUnloadStation` true)
      (break)))
  (if (`self.FoundUnloadStation`)
    (`self.FinishExecute` true)
    (else
      (`self.FinishExecute` false))))