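; Behavior tree service for the robot AI that checks box stations for boxes through the HasBox blackboard key.
; Each tick it gathers all BP_BoxStation actors, printing a blackboard bool for debugging on each iteration.
; The first station with a non-empty BoxArray sets HasBox true and breaks the loop.
; HasBox is then set false after the loop, even following a break.
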(event `self.ReceiveTickAI`
  (params (OwnerController :type "AIController Object Reference") (ControlledPawn :type "Pawn Object Reference") (DeltaSeconds :type "Float (single-precision)"))
  (bind _outactors (`GameplayStatics.GetAllActorsOfClass` "/Game/Blueprint/Item/BP_BoxStation.BP_BoxStation_C"))
  (for _array_element _outactors
    (`KismetSystemLibrary.PrintString` (`KismetStringLibrary.Conv_BoolToString` (`BlackboardComponent.GetValueAsBool` (`AIBlueprintHelperLibrary.GetBlackboard` OwnerController) (`self.Key Name`))))
    (if (> (`KismetArrayLibrary.Array_Length` (`/Game/Blueprint/Item/BP_BoxStation.BoxArray` _array_element)) 0)
      (`BTFunctionLibrary.SetBlackboardValueAsBool` (`self.HasBox`) true)
      (break)))
  (`BTFunctionLibrary.SetBlackboardValueAsBool` (`self.HasBox`)))