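; Behavior tree task for the robot AI that checks whether any box station is available with boxes.
; It gets all BP_BoxStation actors and loops through them, stopping at the first one that is unoccupied and has a non-empty BoxArray.
; Both the found and not-found paths call FinishExecute with false, so the task reports failure in every case.
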(event `CustomEvent`
  (params (OwnerController :type "AIController Object Reference") (ControlledPawn :type "Pawn Object Reference") (DeltaSeconds :type "Float (single-precision)"))
  (bind _outactors (`GameplayStatics.GetAllActorsOfClass` "/Game/Blueprint/Item/BP_BoxStation.BP_BoxStation_C"))
  (for _array_element _outactors
    (bind _boccupied (message `/Game/Blueprint/BPI_Interactable.IsOccupied` _array_element))
    (if (and (not _boccupied) (> (`KismetArrayLibrary.Array_Length` (`/Game/Blueprint/Item/BP_BoxStation.BoxArray` _array_element)) 0))
      (`self.FinishExecute` false)
      (break)))
  (`self.FinishExecute` false))