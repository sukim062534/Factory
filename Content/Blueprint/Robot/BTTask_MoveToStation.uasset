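; Behavior tree task that moves a robot to the TargetLocation blackboard position on the way to its TargetStation.
; It binds the controller's move-completed event once, issues an AI move and finishes successfully when that event reports success.
; Failures from the request or completion share one path that releases a box station's reservation or an unload station's occupancy, clears related blackboard keys and fails the task.
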(event `self.ReceiveExecuteAI`
  (params (OwnerController :type "AIController Object Reference") (ControlledPawn :type "Pawn Object Reference"))
  (bind _returnvalue (`BTFunctionLibrary.GetBlackboardValueAsObject` (`self.TargetStation`)))
  (if (not (`self.bIsBound`))
    (add `AIController.ReceiveMoveCompleted` OwnerController (delegate `OnRobotMoveCompleted`))
    (set `self.bIsBound` true))
  (bind _movementresult (`|AIMoveTo` OwnerController null (`BTFunctionLibrary.GetBlackboardValueAsVector` (`self.TargetLocation`)) null 50.0)
    (:`then`
      (if (not (`|EnumEquality` _movementresult "Success"))
        (bind _asbp_box_station (cast `/Game/Blueprint/Item/BP_BoxStation` _returnvalue :!label _label)
          (:`then`
            (message `/Game/Blueprint/BPI_Interactable.ReleaseReservation` _asbp_box_station)
            (`BTFunctionLibrary.ClearBlackboardValue` (`self.TargetLocation`))
            (`BTFunctionLibrary.ClearBlackboardValue` (`self.TargetStation`))
            (`BTFunctionLibrary.ClearBlackboardValue` (`self.LoadStation`))
            (`self.FinishExecute` false))
          (:`CastFailed`
            (bind _asbp_unload_station (cast `/Game/Blueprint/Item/BP_UnloadStation` _returnvalue)
              (:`then`
                (set `/Game/Blueprint/Item/BP_UnloadStation.bIsOccupied` false _asbp_unload_station)
                (`BTFunctionLibrary.ClearBlackboardValue` (`self.TargetStation`))
                (`self.FinishExecute` false))
              (:`CastFailed`
                (`self.FinishExecute` false)))))))))

(event `OnRobotMoveCompleted`
  (params (RequestID :type "AIRequestID Structure") (Result :type "EPathFollowingResult Enum" :default "Success"))
  (if (`|EnumEquality` Result "Success")
    (`self.FinishExecute` true)
    (else
      (goto _label))))