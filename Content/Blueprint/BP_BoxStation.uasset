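; BP_BoxStation is a station actor that stacks BP_Box actors in a grid when play begins.
; TrySpawnBox calls itself, placing each box at an offset in the Arrow component's space, two by three per layer, based on the BoxArray length.
; It stops when the array holds twelve boxes or the running total reaches SpawnAmount.
; An older spawn chain using actor-location offsets remains disconnected.
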(event `self.ReceiveBeginPlay`
  (`self.TrySpawnBox`))

(event `TrySpawnBox`
  (bind _returnvalue (`KismetArrayLibrary.Array_Length` (`self.BoxArray`)))
  (bind _returnvalue_2 (`|SpawnActorFromClass` "/Game/Blueprint/BP_Box.BP_Box_C" (`KismetMathLibrary.MakeTransform` (`KismetMathLibrary.TransformLocation` (`SceneComponent.K2_GetComponentToWorld` (`self.Arrow`)) (`KismetMathLibrary.MakeVector` (* (mod _returnvalue 2) 100.0) (* (mod (/ _returnvalue 2) 3.0) 75.0) (* (/ _returnvalue 6) 75.0)))) "Undefined" "MultiplyWithRoot" null null))
  (`KismetArrayLibrary.Array_Add` (`self.BoxArray`) _returnvalue_2)
  (set `self.TotalSpawnedCount` (+ (`self.TotalSpawnedCount`) 1))
  (if (and (< (`KismetArrayLibrary.Array_Length` (`self.BoxArray`)) 12) (< (`self.TotalSpawnedCount`) (`self.SpawnAmount`)))
    (`self.TrySpawnBox`)))

(fn `UserConstructionScript`)