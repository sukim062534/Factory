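; Box station that supplies BP_Box actors to robots, with reservation-based access.
; On BeginPlay it recursively spawns boxes in a 2x3x2 grid relative to its Arrow, capped at twelve and by SpawnAmount.
; RequestLoad hands out the last box if the station is unreserved or the requester holds the reservation, without spawning replacements.
; ReleaseReservation clears the reservation and occupied flag, while RequestUnload is a stub returning a zero vector.
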(event `self.ReceiveBeginPlay`
  (`self.TrySpawnBox`))

(event `TrySpawnBox`
  (bind _totalspawnedcount (`self.TotalSpawnedCount`))
  (bind _returnvalue (`|SpawnActorFromClass` "/Game/Blueprint/Item/BP_Box.BP_Box_C" (`KismetMathLibrary.MakeTransform` (`KismetMathLibrary.TransformLocation` (`SceneComponent.K2_GetComponentToWorld` (`self.Arrow`)) (`KismetMathLibrary.MakeVector` (* (mod (mod _totalspawnedcount 12) 2) 100.0) (* (mod (/ (mod _totalspawnedcount 12) 2) 3.0) 75.0) (* (/ (mod _totalspawnedcount 12) 6) 75.0)))) "Undefined" "MultiplyWithRoot" null null))
  (`KismetArrayLibrary.Array_Add` (`self.BoxArray`) _returnvalue)
  (set `self.TotalSpawnedCount` (+ (`self.TotalSpawnedCount`) 1))
  (if (and (< (`KismetArrayLibrary.Array_Length` (`self.BoxArray`)) 12) (< (`self.TotalSpawnedCount`) (`self.SpawnAmount`)))
    (`self.TrySpawnBox`)))

(event `/Game/Blueprint/BPI_Interactable.ReleaseReservation`
  (set `self.ReservedBy` null)
  (set `self.bIsOccupied` false)
  (`KismetSystemLibrary.PrintString` "로봇이 떠났습니다."))

(fn `IsOccupied`
  (returns (bOccupied :type Boolean))
  (return (`self.bIsOccupied`)))

(fn `RequestLoad`
  (params (RequestingRobot :type "/Game/Blueprint/Robot/BP_Robot Object Reference"))
  (returns (GivenBox :type "/Game/Blueprint/Item/BP_Box Object Reference"))
  (bind _boxarray (`self.BoxArray`))
  (bind _returnvalue (`KismetArrayLibrary.Array_LastIndex` _boxarray))
  (`/Engine/EditorBlueprintResources/StandardMacros.IsValid` (`self.ReservedBy`)
    (:`Is Valid`
      (if (== RequestingRobot (`self.ReservedBy`))
        _
        (else
          (return null))))
    (:`Is Not Valid`
      _))
  (if (> (`KismetArrayLibrary.Array_Length` _boxarray) 0)
    (bind _asbp_box (cast `/Game/Blueprint/Item/BP_Box` (`|GetArrayItem` (`self.BoxArray`) _returnvalue)))
    (`KismetArrayLibrary.Array_Remove` (`self.BoxArray`) _returnvalue)
    (return _asbp_box)
    (else
      (return null))))

(fn `RequestUnload`
  (returns (UnloadLocation :type "Vector Structure"))
  (return (0.0 0.0 0.0)))

(fn `UserConstructionScript`)